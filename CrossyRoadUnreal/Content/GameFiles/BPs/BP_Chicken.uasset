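; Player-controlled chicken that hops in steps along four directions.
; Each key press adds a half-step up and forward to a Target location, and each release adds a half-step down and forward.
; Tick feeds Target to MoveComponentTo on the root, while a CanMove flag and short timer ignore inputs that arrive too quickly.
; A gameOver function restarts the current level.
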(event `InputAction|MoveForward`
  (params (Key :type "Key Structure"))
  (:`Pressed`
    (`self.Movement` (50.0 0.0 30.0)))
  (:`Released`
    (`self.Movement` (50.0 0.0 -30.0))))

(event `self.ReceiveTick`
  (params (DeltaSeconds :type "Float (single-precision)"))
  (`KismetSystemLibrary.MoveComponentTo` (`self.DefaultSceneRoot`) (`self.Target`)))

(event `InputAction|MoveBackward`
  (params (Key :type "Key Structure"))
  (:`Pressed`
    (`self.Movement` (-50.0 0.0 30.0)))
  (:`Released`
    (`self.Movement` (-50.0 0.0 -30.0))))

(event `InputAction|MoveLeft`
  (params (Key :type "Key Structure"))
  (:`Pressed`
    (`self.Movement` (0.0 -50.0 30.0)))
  (:`Released`
    (`self.Movement` (0.0 -50.0 -30.0))))

(event `InputAction|MoveRight`
  (params (Key :type "Key Structure"))
  (:`Pressed`
    (`self.Movement` (0.0 50.0 30.0)))
  (:`Released`
    (`self.Movement` (0.0 50.0 -30.0))))

(fn `enableCanMove`
  (set `self.Can Move` true))

(fn `gameOver`
  (bind _returnvalue (`GameplayStatics.GetCurrentLevelName` true))
  (`GameplayStatics.OpenLevel` (`KismetStringLibrary.Conv_StringToName` _returnvalue)))

(fn `Movement`
  (params (direction :type "Vector Structure"))
  (if (`self.Can Move`)
    (set `self.Target` (+ direction (`self.Target`)))
    (set `self.Can Move` false)
    (`KismetSystemLibrary.K2_SetTimer` null "enableCanMove" 0.1)))

(fn `UserConstructionScript`)